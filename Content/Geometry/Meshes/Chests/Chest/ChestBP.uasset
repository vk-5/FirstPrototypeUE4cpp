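; Interactive chest Blueprint whose lid opens and closes on the E key while input is enabled by a trigger box.
; Any overlap with Box enables input for player controller 0, and ending overlap disables it.
; E drives a FlipFlop alternating between the OpenChest and CloseChest events.
; Both use MoveComponentTo to rotate ChestRotator with eased timing, between a tilted open pose and zero relative rotation.
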(event OnComponentBeginOverlap(Box)
  (params (OverlappedComponent :type Primitive%20Component%20Object%20Reference) (OtherActor :type Actor%20Object%20Reference) (OtherComp :type Primitive%20Component%20Object%20Reference) (OtherBodyIndex :type Integer) (bFromSweep :type Boolean) (SweepResult :type Hit%20Result%20Structure%20%28by%20ref%29))
  (Input|EnableInput (Game|GetPlayerController 0)))

(event OnComponentEndOverlap(Box)
  (params (OverlappedComponent :type Primitive%20Component%20Object%20Reference) (OtherActor :type Actor%20Object%20Reference) (OtherComp :type Primitive%20Component%20Object%20Reference) (OtherBodyIndex :type Integer))
  (Input|DisableInput (Game|GetPlayerController 0)))

(event Custom|CloseChest
  (bind _chestrotator (Variables|Default|GetChestRotator))
  (Components|MoveComponentTo _chestrotator (Variables|/Script/Engine.SceneComponent|GetRelativeLocation _chestrotator) "0, 0, 0" true true 1.0 false))

(event Custom|OpenChest
  (bind _chestrotator (Variables|Default|GetChestRotator))
  (Components|MoveComponentTo _chestrotator (Variables|/Script/Engine.SceneComponent|GetRelativeLocation _chestrotator) "0, 0,-110.000000" true true 1.0 false))

(event EventBeginPlay)

(event Collision|EventActorBeginOverlap
  (params (OtherActor :type Actor%20Object%20Reference)))

(event EventTick
  (params (DeltaSeconds :type Float%20%28single-precision%29)))

(event Input|KeyboardEvents|E
  (params (Key :type Key%20Structure))
  (:Pressed
    (Utilities|FlowControl|FlipFlop
      (:A
        (CallFunction|OpenChest))
      (:B
        (CallFunction|CloseChest)))))

(fn ConstructionScript)